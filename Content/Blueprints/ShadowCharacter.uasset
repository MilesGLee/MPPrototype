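; Player character with a camera-relative walk mode and an E-toggled "diving" mode that turns off gravity and switches to flying.
; Tick applies movement, rotates the pitch-clamped spring arm, and eases mesh and orientation toward camera yaw when not diving.
; While diving, velocity is damped and input follows stored direction vectors.
; A short forward trace adopts the hit actor's forward and up vectors during forward input, snapping orientation and mesh rotation.
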(event `ApplyCameraRotation`
  (bind _cameraspringarm (`self.CameraSpringArm`))
  (bind (_relativerotation_roll _relativerotation_pitch _relativerotation_yaw) (`KismetMathLibrary.BreakRotator` (`SceneComponent.RelativeRotation` _cameraspringarm)))
  ;[1 1 1] Comment
  (`SceneComponent.K2_AddRelativeRotation` _cameraspringarm (`KismetMathLibrary.MakeRotator` 0.0 (`self.InputMouseVertical`) (`self.InputMouseHorizontal`)) false false)
  (`SceneComponent.K2_SetRelativeRotation` _cameraspringarm (`KismetMathLibrary.MakeRotator` 0.0 (`KismetMathLibrary.FClamp` _relativerotation_pitch -70.0 70.0) _relativerotation_yaw) false false))

(event `ApplyOrientationRotation`
  (bind (_relativerotation_roll _relativerotation_pitch _relativerotation_yaw) (`KismetMathLibrary.BreakRotator` (`SceneComponent.RelativeRotation` (`self.CameraSpringArm`))))
  ;[1 1 1] Rotate Orientation
  (if (not (`self.IsDiving`))
    (`SceneComponent.K2_SetRelativeRotation` (`self.Orientation`) (`KismetMathLibrary.RLerp` (`SceneComponent.RelativeRotation` (`self.Orientation`)) (`KismetMathLibrary.MakeRotator` 0.0 0.0 _relativerotation_yaw) 0.05 true) false false)))

(event `ApplyMovement`
  ;[1 1 1] Character Movement
  (if (not (`self.IsDiving`))
    (`self.AddMovementInput` (`KismetMathLibrary.Normal` (* (`SceneComponent.GetForwardVector` (`self.Camera`)) (`self.InputVertical`))) 100.0)
    (`self.AddMovementInput` (`KismetMathLibrary.Normal` (* (`SceneComponent.GetRightVector` (`self.Camera`)) (`self.InputHorizontal`))) 100.0)
    (else
      (set `MovementComponent.Velocity` (/ (`MovementComponent.Velocity` (`self.CharacterMovement`)) 1.05) (`self.CharacterMovement`))
      (`self.AddMovementInput` (`KismetMathLibrary.Normal` (* (`self.ForwardVector`) (* 1 (`self.InputVertical`)))) 100.0)
      (`self.AddMovementInput` (`KismetMathLibrary.Normal` (* (`self.RightVector`) (`self.InputHorizontal`))) 100.0))))

(event `ApplyMeshRotation`
  (bind (_relativerotation_roll _relativerotation_pitch _relativerotation_yaw) (`KismetMathLibrary.BreakRotator` (`SceneComponent.RelativeRotation` (`self.CameraSpringArm`))))
  ;[1 1 1] Rotate mesh to match moving direction
  (if (not (`self.IsDiving`))
    (`SceneComponent.K2_SetRelativeRotation` (`self.Mesh`) (`KismetMathLibrary.RLerp` (`SceneComponent.RelativeRotation` (`self.Mesh`)) (`KismetMathLibrary.MakeRotator` 0.0 0.0 (+ -90.0 _relativerotation_yaw)) 0.05 true) false false)))

(event `Key|E`
  (params (Key :type "Key Structure"))
  (bind _charactermovement (`self.CharacterMovement`))
  (bind _charactermovement_2 (`self.CharacterMovement`))
  (:`Pressed`
    (set `self.IsDiving` (not (`self.IsDiving`)))
    (if (`self.IsDiving`)
      (`CharacterMovementComponent.SetMovementMode` _charactermovement_2 "MOVE_Flying" 0)
      (set `CharacterMovementComponent.GravityScale` 0.0 _charactermovement_2)
      (else
        (set `self.ForwardVector` (1.0 0.0 0.0))
        (set `self.UpVector` (0.0 0.0 1.0))
        (set `self.RightVector` (0.0 1.0 0.0))
        (`CharacterMovementComponent.SetMovementMode` _charactermovement "MOVE_Walking" 0)
        (set `CharacterMovementComponent.GravityScale` 1.0 _charactermovement)))))

(event `Key|LeftShift`
  (params (Key :type "Key Structure")))

(event `self.ReceiveBeginPlay`
  (set `self.ForwardVector` (1.0 0.0 0.0))
  (set `self.UpVector` (0.0 0.0 1.0))
  (set `self.RightVector` (0.0 1.0 0.0)))

(event `self.ReceiveTick`
  (params (DeltaSeconds :type "Float (single-precision)"))
  (bind _orientation (`self.Orientation`))
  (bind (_forwardray_bblockinghit _forwardray_binitialoverlap _forwardray_time _forwardray_distance _forwardray_location _forwardray_impactpoint _forwardray_normal _forwardray_impactnormal _forwardray_physmat _forwardray_hitactor) (`GameplayStatics.BreakHitResult` (`self.ForwardRay`)))
  (bind _returnvalue (`SceneComponent.K2_GetComponentLocation` _orientation))
  (`self.ApplyMovement`)
  (`self.ApplyCameraRotation`)
  (`self.ApplyMeshRotation`)
  (`self.ApplyOrientationRotation`)
  (`KismetSystemLibrary.PrintString` (`KismetStringLibrary.Conv_VectorToString` (`self.ForwardVector`)))
  (if (`self.IsDiving`)
    (bind (_outhit _returnvalue_2) (`KismetSystemLibrary.LineTraceSingle` :`Start` _returnvalue :`End` (+ _returnvalue (* (`SceneComponent.GetForwardVector` _orientation) 45.0)) :`TraceChannel` "TraceTypeQuery1" :`DrawDebugType` "ForDuration"))
    (set `self.ForwardRay` _outhit)
    (if (and _returnvalue_2 (> (`self.InputVertical`) 0.0))
      (bind _output_get (set `self.ForwardVector` (`self.GetActorForwardVector` _forwardray_hitactor)))
      (set `self.UpVector` (`self.GetActorUpVector` _forwardray_hitactor))
      (bind _returnvalue_3 (`KismetMathLibrary.Conv_VectorToRotator` _output_get))
      (`SceneComponent.K2_SetRelativeRotation` (`self.Orientation`) (* _returnvalue_3 -1.0) false false)
      (`SceneComponent.K2_SetRelativeRotation` (`self.Mesh`) _returnvalue_3 false false))))

(event `InputAxis|Horizontal`
  (params (AxisValue :type "Float (single-precision)"))
  (set `self.InputHorizontal` AxisValue))

(event `InputAxis|Vertical`
  (params (AxisValue :type "Float (single-precision)"))
  (set `self.InputVertical` AxisValue))

(event `InputAxis|MouseHorizontal`
  (params (AxisValue :type "Float (single-precision)"))
  (set `self.InputMouseHorizontal` AxisValue))

(event `InputAxis|MouseVertical`
  (params (AxisValue :type "Float (single-precision)"))
  (set `self.InputMouseVertical` AxisValue))

(fn `UserConstructionScript`)