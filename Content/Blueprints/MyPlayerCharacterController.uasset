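; Player character controller Blueprint that turns axis input into movement and look rotation.
; Axis events cache keyboard-style and mouse values in variables, which Tick passes every frame to ApplyMovement and ApplyLookRotation with fixed speeds.
; Both functions are called here but defined outside this file.
; Jump and StartDash calls are present but unconnected, so neither runs.
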(event `self.ReceiveBeginPlay`)

(event `self.ReceiveTick`
  (params (DeltaSeconds :type "Float (single-precision)"))
  (`self.ApplyMovement` (`self.inputHorizontal`) (`self.inputVertical`) 10.0)
  (`self.ApplyLookRotation` (`self.inputMouseHorizontal`) (`self.inputMouseVertical`) 10.0))

(event `InputAxis|Horizontal`
  (params (AxisValue :type "Float (single-precision)"))
  (set `self.inputHorizontal` AxisValue))

(event `InputAxis|Vertical`
  (params (AxisValue :type "Float (single-precision)"))
  (set `self.inputVertical` AxisValue))

(event `InputAxis|MouseHorizontal`
  (params (AxisValue :type "Float (single-precision)"))
  (set `self.inputMouseHorizontal` AxisValue))

(event `InputAxis|MouseVertical`
  (params (AxisValue :type "Float (single-precision)"))
  (set `self.inputMouseVertical` AxisValue))

(event `InputAction|Jump`
  (params (Key :type "Key Structure")))

(event `InputAction|Dash`
  (params (Key :type "Key Structure")))

(fn `UserConstructionScript`)